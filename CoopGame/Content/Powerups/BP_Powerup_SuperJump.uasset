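; Super Jump powerup Blueprint that temporarily doubles a player's jump height velocity while active.
; On activation it stores the target player and multiplies its CharacterMovementComponent JumpZVelocity by two.
; On expiry it halves that velocity if the stored player is still valid, then always runs the parent expiry logic.
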(event `self.OnActivated`
  (params (ActivateFor :type "Actor Object Reference"))
  (bind _returnvalue (`self.GetComponentByClass` ActivateFor "/Script/Engine.CharacterMovementComponent"))
  (set `self.ActivatedForPlayer` ActivateFor)
  (set `CharacterMovementComponent.JumpZVelocity` (* (`CharacterMovementComponent.JumpZVelocity` _returnvalue) 2.0) _returnvalue))

(event `self.OnExpired`
  (bind _activatedforplayer (`self.ActivatedForPlayer`))
  (bind _returnvalue (`self.GetComponentByClass` _activatedforplayer "/Script/Engine.CharacterMovementComponent"))
  (`/Engine/EditorBlueprintResources/StandardMacros.IsValid` _activatedforplayer
    (:`Is Valid`
      (set `CharacterMovementComponent.JumpZVelocity` (/ (`CharacterMovementComponent.JumpZVelocity` _returnvalue) 2.0) _returnvalue)
      (`parent.OnExpired`))
    (:`Is Not Valid`
      (`parent.OnExpired`))))

(fn `UserConstructionScript`
  (`parent.UserConstructionScript`))