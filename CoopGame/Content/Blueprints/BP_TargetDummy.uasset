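; BP_TargetDummy is a target dummy actor that visualizes the damage it receives for debugging.
; Point and radial damage events each print the amount and briefly draw a red debug sphere at the hit location or blast origin.
; Point damage also shows the amount as green text above the actor, while the radial event's matching debug string has no text input connected.
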(event `self.ReceivePointDamage`
  (params (Damage :type "Float (single-precision)") (DamageType :type "DamageType Object Reference") (HitLocation :type "Vector Structure") (HitNormal :type "Vector Structure") (HitComponent :type "PrimitiveComponent Object Reference") (BoneName :type Name) (ShotFromDirection :type "Vector Structure") (InstigatedBy :type "Controller Object Reference") (DamageCauser :type "Actor Object Reference") (HitInfo :type "HitResult Structure (by ref)"))
  (`KismetSystemLibrary.PrintString` (`KismetStringLibrary.Conv_DoubleToString` Damage))
  (`KismetSystemLibrary.DrawDebugSphere` HitLocation 10.0 6 (struct :`R` 1.0 :`A` 1.0) 1.0 1.0)
  (`KismetSystemLibrary.DrawDebugString` (+ (`self.K2_GetActorLocation`) (-50.0 0.0 200.0)) (`KismetStringLibrary.Conv_DoubleToString` Damage) null (struct :`G` 1.0 :`A` 1.0) 1.0))

(event `self.ReceiveRadialDamage`
  (params (DamageReceived :type "Float (single-precision)") (DamageType :type "DamageType Object Reference") (Origin :type "Vector Structure") (HitInfo :type "HitResult Structure (by ref)") (InstigatedBy :type "Controller Object Reference") (DamageCauser :type "Actor Object Reference"))
  (`KismetSystemLibrary.PrintString` (`KismetStringLibrary.Conv_DoubleToString` DamageReceived))
  (`KismetSystemLibrary.DrawDebugSphere` Origin 10.0 6 (struct :`R` 1.0 :`A` 1.0) 1.0 1.0)
  (`KismetSystemLibrary.DrawDebugString` (+ (`self.K2_GetActorLocation`) (-50.0 0.0 200.0)) "" null (struct :`G` 1.0 :`A` 1.0) 1.0))

(fn `UserConstructionScript`)